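; MainmenuGM, apparently the main menu's game mode, shows the Mainmenu widget when play begins.
; BeginPlay creates the widget, stores it, adds it to the viewport and passes it to SetWidgetInput.
; That function switches the first player controller to Game and UI input focused on the widget and shows the mouse cursor.
; Tick is empty, and a leftover cursor node in the event graph is unconnected.
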(event `self.ReceiveBeginPlay`
  (bind _returnvalue (`|CreateWidget` "/Game/UI/Mainmenu.Mainmenu_C"))
  (bind _output_get (set `self.NewVar_0` _returnvalue))
  (`UserWidget.AddToViewport` _output_get 0)
  (`self.SetWidgetInput` (`self.NewVar_0`)))

(fn `SetWidgetInput`
  (params (InWidgetToFocus :type "Widget Object Reference"))
  (bind _returnvalue (`GameplayStatics.GetPlayerController` 0))
  (`WidgetBlueprintLibrary.SetInputMode_GameAndUIEx` _returnvalue InWidgetToFocus "DoNotLock" false)
  (set `PlayerController.bShowMouseCursor` true _returnvalue))

(fn `UserConstructionScript`)