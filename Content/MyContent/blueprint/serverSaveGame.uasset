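; Server save-game Blueprint, going by its name, that keeps a per-player kill tally.
; Player names and kill counts live in parallel arrays, with AddPlayer appending a zero-kill entry only for names not already present.
; AddKill finds the index by linear name search, increments that count and prints a debug message, without checking that the player exists.
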(fn `addKill`
  (params (playerName :type String))
  (bind _playerskills (`self.playersKills`))
  (bind _playerindex (`self.getPlayerIndex` playerName))
  (bind _returnvalue (+ (`|GetArrayItem` _playerskills _playerindex) 1))
  (`KismetArrayLibrary.Array_Set` _playerskills _playerindex _returnvalue)
  (`KismetSystemLibrary.PrintString` null (`KismetStringLibrary.Concat_StrStr` "Player kills incremented: " (`KismetStringLibrary.Conv_IntToString` _returnvalue))))

(fn `addPlayer`
  (params (playerName :type String))
  ;[1 1 1] Add player if isn't already present
  (bind _ispresent (`self.checkIfPlayerIsAlreadyPresent` playerName))
  (if (not _ispresent)
    (`KismetArrayLibrary.Array_Add` (`self.playersName`) playerName)
    (`KismetArrayLibrary.Array_Add` (`self.playersKills`))))

(fn `checkIfPlayerIsAlreadyPresent`
  (params (playerName :type String))
  (returns (isPresent :type Boolean))
  (for _array_element (`self.playersName`)
    (if (`KismetStringLibrary.EqualEqual_StrStr` _array_element playerName)
      (`|ExecutionSequence`
        (:`then_0`
          (break))
        (:`then_1`
          (return true)))))
  (return false))

(fn `getPlayerIndex`
  (params (playerName :type String))
  (returns (playerIndex :type Integer))
  (for (_array_element _array_index) (`self.playersName`)
    (if (`KismetStringLibrary.EqualEqual_StrStr` playerName _array_element)
      (`|ExecutionSequence`
        (:`then_0`
          (break))
        (:`then_1`
          (return _array_index))))))