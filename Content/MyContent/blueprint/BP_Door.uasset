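; Networked swinging door that opens on character overlap, either automatically on the server or through an interact prompt, and can be preset open in the editor.
; The overlap tracks players and hands each a door reference; DoorOpen picks a swing sign from location-vector lengths and plays the OpenDoor timeline.
; The timeline reverses when the last player leaves.
; A rep-notify on the open state toggles the prompt widget for local players in range.
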(event `self.ReceiveBeginPlay`
  (set `self.defaultRotation` (`SceneComponent.RelativeRotation` (`self.Door`))))

(event `self.DoorCollision.OnComponentBeginOverlap`
  (params (OverlappedComponent :type "PrimitiveComponent Object Reference") (OtherActor :type "Actor Object Reference") (OtherComp :type "PrimitiveComponent Object Reference") (OtherBodyIndex :type Integer) (bFromSweep :type Boolean) (SweepResult :type "HitResult Structure (by ref)"))
  (`/Engine/EditorBlueprintResources/StandardMacros.IsValid` OtherActor
    (:`Is Valid`
      (bind _asthird_person_character (cast `/Game/ThirdPersonBP/Blueprints/ThirdPersonCharacter` OtherActor))
      (bind _output_get (set `self.player` _asthird_person_character))
      (`KismetArrayLibrary.Array_Add` (`self.players`) _output_get)
      (set `/Game/ThirdPersonBP/Blueprints/ThirdPersonCharacter.Door1` self (`self.player`))
      (if (not (`self.bInteract?`))
        (`/Engine/EditorBlueprintResources/ActorMacros.Switch Has Authority`
          (:`Authority`
            (`self.DoorOpen` (`self.player`))))
        (else
          (`self.AddOpenDoorUItoScreen` (`self.player`)))))))

(event `self.DoorCollision.OnComponentEndOverlap`
  (params (OverlappedComponent :type "PrimitiveComponent Object Reference") (OtherActor :type "Actor Object Reference") (OtherComp :type "PrimitiveComponent Object Reference") (OtherBodyIndex :type Integer))
  (`/Engine/EditorBlueprintResources/StandardMacros.IsValid` OtherActor
    (:`Is Valid`
      (bind _asthird_person_character (cast `/Game/ThirdPersonBP/Blueprints/ThirdPersonCharacter` OtherActor))
      (bind _output_get (set `self.player` _asthird_person_character))
      (`KismetArrayLibrary.Array_RemoveItem` (`self.players`) _output_get)
      (`self.RemoveOpenDoorUI` (`self.player`))
      (if (== (`KismetArrayLibrary.Array_Length` (`self.players`)) 0)
        (`TimelineComponent.Reverse` (`self.OpenDoor`))
        (set `self.isDoorOpen` false)))))

(event `DoorOpen`
  (params (player :type "/Game/ThirdPersonBP/Blueprints/ThirdPersonCharacter Object Reference"))
  ;[1 1 1] Door Open
  (set `self.player` player)
  (if (not (`self.isDoorOpen`))
    (if (not (`TimelineComponent.IsPlaying` (`self.OpenDoor`))) :!label _label
      (set `self.direction` (`self.GetDoorSwingDirection` (`self.player`)))
      (`TimelineComponent.Play` (`self.OpenDoor`))
      (set `self.isDoorOpen` true)
      (else
        (`KismetSystemLibrary.Delay` 0.2)
        (goto _label)))))

(fn `AddOpenDoorUItoScreen`
  (params (player :type "/Game/ThirdPersonBP/Blueprints/ThirdPersonCharacter Object Reference"))
  (bind _returnvalue (`Pawn.GetController` player))
  (`/Engine/EditorBlueprintResources/StandardMacros.IsValid` _returnvalue
    (:`Is Valid`
      (if (`Controller.IsLocalPlayerController` _returnvalue)
        (bind _returnvalue_2 (`|CreateWidget` "/Game/UI/EInteractOpenDoor.EInteractOpenDoor_C" (cast `/Game/ThirdPersonBP/Blueprints/MyPlayerController` _returnvalue :!pure true)))
        (bind _output_get (set `self.interactUI` _returnvalue_2))
        (`UserWidget.AddToViewport` _output_get 0)))))

(fn `GetDoorSwingDirection`
  (params (player :type "/Game/ThirdPersonBP/Blueprints/ThirdPersonCharacter Object Reference"))
  (returns (direction :type "Float (double-precision)"))
  (`/Engine/EditorBlueprintResources/StandardMacros.IsValid` player
    (:`Is Valid`
      (return (`KismetMathLibrary.FClamp` (- (`KismetMathLibrary.VSize` (`self.K2_GetActorLocation` player)) (`KismetMathLibrary.VSize` (`SceneComponent.K2_GetComponentLocation` (`self.Door`)))) 1.0 -1.0)))
    (:`Is Not Valid`
      (return 0.0))))

(fn `OnRep_isDoorOpen`
  (bind _interactui (`self.interactUI`))
  (if (`self.isDoorOpen`)
    (for _array_element (`self.players`)
      (bind _returnvalue (`Pawn.GetController` _array_element))
      (`/Engine/EditorBlueprintResources/StandardMacros.IsValid` _returnvalue
        (:`Is Valid`
          (if (`Controller.IsLocalPlayerController` _returnvalue)
            (`/Engine/EditorBlueprintResources/StandardMacros.IsValid` _interactui
              (:`Is Valid`
                (`Widget.RemoveFromParent` _interactui)))))))
    (else
      (for _array_element_2 (`self.players`)
        (bind _returnvalue_2 (`Pawn.GetController` _array_element_2))
        (`/Engine/EditorBlueprintResources/StandardMacros.IsValid` _returnvalue_2
          (:`Is Valid`
            (if (`Controller.IsLocalPlayerController` _returnvalue_2)
              (bind _returnvalue_3 (`|CreateWidget` "/Game/UI/EInteractOpenDoor.EInteractOpenDoor_C" (cast `/Game/ThirdPersonBP/Blueprints/MyPlayerController` _returnvalue_2 :!pure true)))
              (bind _output_get (set `self.interactUI` _returnvalue_3))
              (`UserWidget.AddToViewport` _output_get 0))))))))

(fn `RemoveOpenDoorUI`
  (params (player :type "/Game/ThirdPersonBP/Blueprints/ThirdPersonCharacter Object Reference"))
  (bind _returnvalue (`Pawn.GetController` player))
  (bind _interactui (`self.interactUI`))
  (`/Engine/EditorBlueprintResources/StandardMacros.IsValid` _returnvalue
    (:`Is Valid`
      (if (`Controller.IsLocalPlayerController` _returnvalue)
        (`/Engine/EditorBlueprintResources/StandardMacros.IsValid` _interactui
          (:`Is Valid`
            (`Widget.RemoveFromParent` _interactui)
            (set `self.interactUI` null)))))))

(fn `UserConstructionScript`
  (if (`self.bOpen`)
    (`SceneComponent.K2_SetRelativeRotation` (`self.Door`) (select `bool` (`self.bPositiviDirection`) :`false` (struct :`Yaw` -90.0) :`true` (struct :`Yaw` 90.0) :!type "Rotator Structure") false false)
    (else
      (`SceneComponent.K2_SetRelativeRotation` :`self` (`self.Door`)))))